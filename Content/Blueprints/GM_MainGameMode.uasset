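; GM_MainGameMode is the main game mode, running the match countdown and ending play with a scoreboard.
; A Delay on Tick serves as a one-second timer that decrements Seconds and rolls over into Minutes.
; When a rollover brings Minutes to zero or below, it pauses the game, casts the player character to BP_MainPlayerCharacter and adds WBP_Scoreboard to the viewport.
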(event `self.ReceiveTick`
  (params (DeltaSeconds :type "Float (single-precision)"))
  (`KismetSystemLibrary.Delay` 1.0)
  (set `self.Seconds` (- (`self.Seconds`) 1))
  (if (< (`self.Seconds`) 0)
    (set `self.Seconds` 59)
    (set `self.Minutes` (- (`self.Minutes`) 1))
    (if (<= (`self.Minutes`) 0)
      (`GameplayStatics.SetGamePaused` true)
      (cast `/Game/Blueprints/MainPlayer/BP_MainPlayerCharacter` (`GameplayStatics.GetPlayerCharacter` 0))
      (bind _returnvalue (`|CreateWidget` "/Game/Blueprints/Widgets/Gameplay/WBP_Scoreboard.WBP_Scoreboard_C"))
      (`UserWidget.AddToViewport` _returnvalue 0))))

(fn `UserConstructionScript`)