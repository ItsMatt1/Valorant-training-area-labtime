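; BP_MainHUD is the game's main HUD, exposing toggles for the scoreboard, armor damage and health damage visuals.
; Each function looks up "MainGameWidget" by name, casts it to WBP_MainGameWidget and forwards the Active flag to that widget.
; The scoreboard and armor toggles return true on success, while the health damage toggle returns false.
; The event graph and construction script are empty.
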(event `self.ReceiveBeginPlay`)

(fn `ToggleArmorDamageWidget`
  (params (bActive :type Boolean))
  (returns (ReturnValue :type Boolean))
  ;[1 1 1] Get the main game widget
  (bind _returnvalue (`self.GetWidgetByName` "MainGameWidget")
    (:`Found`
      (bind _aswbp_main_game_widget (cast `/Game/Blueprints/Widgets/Gameplay/WBP_MainGameWidget` _returnvalue))
      ;[1 1 1] Toggle scoreboard widget inside of it
      (`/Game/Blueprints/Widgets/Gameplay/WBP_MainGameWidget.Toggle ArmorDamageVisualization` _aswbp_main_game_widget bActive)
      (return true))))

(fn `ToggleDamageWidget`
  (params (bActive :type Boolean))
  (returns (ReturnValue :type Boolean))
  ;[1 1 1] Get the main game widget
  (bind _returnvalue (`self.GetWidgetByName` "MainGameWidget")
    (:`Found`
      (bind _aswbp_main_game_widget (cast `/Game/Blueprints/Widgets/Gameplay/WBP_MainGameWidget` _returnvalue))
      ;[1 1 1] Toggle scoreboard widget inside of it
      (`/Game/Blueprints/Widgets/Gameplay/WBP_MainGameWidget.Toggle Health Damage Effect` _aswbp_main_game_widget bActive)
      (return false))))

(fn `ToggleScoreboardWidget`
  (params (bActive :type Boolean))
  (returns (ReturnValue :type Boolean))
  ;[1 1 1] Get the main game widget
  (bind _returnvalue (`self.GetWidgetByName` "MainGameWidget")
    (:`Found`
      (bind _aswbp_main_game_widget (cast `/Game/Blueprints/Widgets/Gameplay/WBP_MainGameWidget` _returnvalue))
      ;[1 1 1] Toggle scoreboard widget inside of it
      (`/Game/Blueprints/Widgets/Gameplay/WBP_MainGameWidget.Toggle ScoreboardVisualization` _aswbp_main_game_widget bActive)
      (return true))))

(fn `UserConstructionScript`)