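; Enemy character that spawns behind a fire effect, staying hidden briefly, then repeatedly damages the player and reacts to bullet hits.
; After a start delay, Tick applies damage and camera shake on a DoDamage cooldown, with no range check.
; Bullet hits show a hitmarker and read HealthComponent, either playing a small explosion or broadcasting EnemyKilled, showing a kill popup and destroying the actor.
; BeginPlay also calls UpdateEnemiesKilledAmount on BP_MainPlayerState.
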(event `self.ReceiveBeginPlay`
  (`GameplayStatics.PlaySound2D` "/Game/Sounds/A_Spawn_15.A_Spawn_15" 1.0 1.0 0.0 null null)
  (bind _returnvalue (`GameplayStatics.GetActorOfClass` "/Game/Blueprints/BP_MainPlayerState.BP_MainPlayerState_C"))
  (`MainPlayerState.UpdateEnemiesKilledAmount` _returnvalue)
  (`GameplayStatics.SpawnEmitterAttached` "/Game/InfinityBladeEffects/Effects/FX_Mobile/Fire/combat/P_AOE_Fire_CircleAttack.P_AOE_Fire_CircleAttack" (`self.Mesh`) "ik_foot_root" (`CharacterMovementComponent.GetLastUpdateLocation` (`self.CharacterMovement`)))
  (`SceneComponent.SetVisibility` (`self.Mesh`) false false)
  (`SceneComponent.SetVisibility` (`self.CapsuleComponent`) false false)
  (`KismetSystemLibrary.Delay` 1.15)
  (`SceneComponent.SetVisibility` (`self.Mesh`) true false)
  (`SceneComponent.SetVisibility` (`self.CapsuleComponent`) true false)
  (`KismetSystemLibrary.Delay` 3.0)
  (set `self.bDoDamage` true))

(event `self.ReceiveAnyDamage`
  (params (Damage :type "Float (single-precision)") (DamageType :type "DamageType Object Reference") (InstigatedBy :type "Controller Object Reference") (DamageCauser :type "Actor Object Reference"))
  (set `self.Damage` Damage))

(event `self.ReceiveTick`
  (params (DeltaSeconds :type "Float (single-precision)"))
  (if (`self.bDoDamage`)
    (bind _asbp_main_player_character (cast `/Game/Blueprints/MainPlayer/BP_MainPlayerCharacter` (`GameplayStatics.GetPlayerCharacter` 0)))
    (`MainPlayerCharacter.TakeDamageFromEnemy` _asbp_main_player_character)
    (`GameplayStatics.ApplyDamage` _asbp_main_player_character 15.0)
    (set `self.bDoDamage` false)
    (`GameplayStatics.PlayWorldCameraShake` "/Game/Blueprints/BP_MyCameraShake.BP_MyCameraShake_C" (`self.K2_GetActorLocation` _asbp_main_player_character) 0.0 80.0)
    (`KismetSystemLibrary.Delay` 1.2)
    (set `self.bDoDamage` true)))

(event `self.EnemyHitByBulletEvent`
  (`self.On Hit by Bullet`))

(fn `On Hit by Bullet`
  (bind _health (`HealthComponent.Health` (`self.HealthComponent`)))
  (bind _returnvalue (`|CreateWidget` "/Game/Blueprints/Widgets/Hud/WBP_Hitmarker.WBP_Hitmarker_C"))
  (`UserWidget.AddToViewport` _returnvalue 0)
  (`KismetSystemLibrary.PrintString` (`KismetStringLibrary.Conv_DoubleToString` _health))
  (if (<= _health 0.0)
    (`self.EnemyKilled`)
    (bind _returnvalue_2 (`|CreateWidget` "/Game/Blueprints/Widgets/Hud/WBP_KillPopup.WBP_KillPopup_C"))
    (`UserWidget.AddToViewport` _returnvalue_2 0)
    (clear `self.EnemyKilled`)
    (`self.K2_DestroyActor`)
    (else
      (`GameplayStatics.SpawnEmitterAtLocation` "/Game/InfinityBladeEffects/Effects/FX_Monsters/FX_Monster_Gruntling/Bomber/P_FireBombExplosion.P_FireBombExplosion" (`self.K2_GetActorLocation` self) (`self.K2_GetActorRotation` self) (0.2 0.2 0.2)))))

(fn `UserConstructionScript`)