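; Player character Blueprint that creates the FPS HUD and a weapon on BeginPlay, attaching the weapon to a mesh socket and firing it on PrimaryFire.
; Tick uses a Delay to regenerate Armor in small steps, roughly once per second while below full.
; TakeDamage15 subtracts fixed damage from Armor, carries any overflow into Health, and shows either a health or armor damage effect widget.
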(event `InputAction|PrimaryFire`
  (params (Key :type "Key Structure"))
  (:`Pressed`
    (`/Game/Blueprints/Weapons/AK-47/Weapon_Base.Fire` (`self.EquippedWeapon`))))

(event `self.ReceiveBeginPlay`
  (bind _returnvalue (`|CreateWidget` "/Game/Blueprints/MainPlayer/FPSHud.FPSHud_C"))
  (`UserWidget.AddToViewport` _returnvalue 0)
  (bind _returnvalue_2 (`|SpawnActorFromClass` "/Game/Blueprints/Weapons/AK-47/Weapon_Base.Weapon_Base_C" (`KismetMathLibrary.MakeTransform` (0.0 0.0 0.0)) "Undefined" "OverrideRootScale" null null))
  (bind _output_get (set `self.EquippedWeapon` _returnvalue_2))
  (`self.K2_AttachToComponent` _output_get (`self.Mesh`) "Weapon_Attach" "KeepRelative" "KeepRelative" "KeepRelative" true))

(event `self.ReceiveTick`
  (params (DeltaSeconds :type "Float (single-precision)"))
  (`|ExecutionSequence`
    (:`then_0`
      (`KismetSystemLibrary.Delay` 1.0)
      (if (< (`self.Armor`) 1.0)
        (set `self.Armor` (+ (`self.Armor`) 0.01))))))

(fn `TakeDamage15%`
  (bind _output_get (set `self.Armor` (- (`self.Armor`) 0.15)))
  (if (< _output_get 0.0)
    (set `self.Health` (+ (`self.Armor`) (`self.Health`)))
    (set `self.Armor` 0.0)
    (bind _returnvalue (`|CreateWidget` "/Game/Blueprints/MainPlayer/DamageEffect.DamageEffect_C" (`GameplayStatics.GetPlayerController` 0)))
    (`UserWidget.AddToViewport` _returnvalue 0)
    (else
      (bind _returnvalue_2 (`|CreateWidget` "/Game/Blueprints/MainPlayer/ArmorDamageEffect.ArmorDamageEffect_C" (`GameplayStatics.GetPlayerController` 0)))
      (`UserWidget.AddToViewport` _returnvalue_2 0))))

(fn `UserConstructionScript`)