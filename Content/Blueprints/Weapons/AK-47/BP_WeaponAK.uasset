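; AK-47 weapon Blueprint with a FireAutomatic event for hitscan firing, though every node in that event is disabled.
; The disabled logic plays a shot sound, then line-traces from the player's ADS or follow camera depending on aiming state.
; Each branch decrements the player's AK ammo, spawns a scaled-down muzzle flash at the weapon socket and notifies any BP_TargetEnemy hit.
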(fn `UserConstructionScript`)